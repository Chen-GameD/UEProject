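; BP_DamageActor is a trigger hazard that damages and temporarily slows a UEMainCharacter entering its Box component.
; On overlap, it lowers health through the character's UEPlayerState by the Damage amount.
; It then sets ForwardMoveSpeed on player controller 0 to SlowDownSpeed and, after a five-second Delay, restores a hard-coded speed rather than the previous one.
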(event OnComponentBeginOverlap(Box)
  (params (OverlappedComponent :type Primitive%20Component%20Object%20Reference) (OtherActor :type Actor%20Object%20Reference) (OtherComp :type Primitive%20Component%20Object%20Reference) (OtherBodyIndex :type Integer) (bFromSweep :type Boolean) (SweepResult :type Hit%20Result%20Structure%20%28by%20ref%29))
  (bind _asuemain_character (Utilities|Casting|CastToUEMainCharacter OtherActor))
  (bind _asueplayer_state (Utilities|Casting|CastToUEPlayerState (Variables|/Script/Engine.Pawn|GetPlayerState _asuemain_character)))
  (Default|DecreaseHealth _asueplayer_state (Variables|Default|GetDamage))
  (Utilities|Casting|CastToUEMainCharacter OtherActor)
  (bind _asueplayer_controller (Utilities|Casting|CastToUEPlayerController (Game|GetPlayerController 0)))
  (Variables|/Game/Gameplay/BP/Basis/UEPlayerController.UEPlayerController_C|SetForwardMoveSpeed _asueplayer_controller (Variables|Default|GetSlowDownSpeed))
  (Utilities|FlowControl|Delay 5.0)
  (Variables|/Game/Gameplay/BP/Basis/UEPlayerController.UEPlayerController_C|SetForwardMoveSpeed _asueplayer_controller 4e+02))

(event EventBeginPlay)

(event Collision|EventActorBeginOverlap
  (params (OtherActor :type Actor%20Object%20Reference)))

(event EventTick
  (params (DeltaSeconds :type Float%20%28single-precision%29)))

(fn ConstructionScript)